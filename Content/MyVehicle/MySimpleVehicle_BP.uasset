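; Simple wheeled vehicle Blueprint with differential (skid-steer) driving, controlled by player input or MQTT messages.
; A 60 Hz loop runs PID controllers on linear and yaw velocity to set per-wheel torques, charting yaw rate in a web widget.
; Manual mode publishes measured velocity as cmd_vel.
; Remote mode follows odometry JSON targets, returning to idle with a brake reset after a half-second timeout; mode changes are published.
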(event `self.ReceiveBeginPlay`
  (bind _returnvalue (`|CreateWidget` "/Game/MyVehicle/Figure.Figure_C"))
  (`UserWidget.AddToViewport` _returnvalue 0)
  (set `self.Figure` _returnvalue)
  (`KismetSystemLibrary.K2_SetTimerDelegate` (delegate `LoopInFixedTime0`) 0.016667 true)
  (`KismetSystemLibrary.K2_SetTimerDelegate` (delegate `LoopInFixedTime1`) 0.1 true))

(event `LoopInFixedTime0`
  (`self.Main`))

(event `LoopInFixedTime1`
  (bind _linear_x (`KismetMathLibrary.BreakVector` (`self.Linear`)))
  (bind (_angular_x _angular_y _angular_z) (`KismetMathLibrary.BreakVector` (`self.Angular`)))
  (if (!= (`self.ControlMode`) 1)
    (if (== (`self.ControlMode`) 2)
      (if (>= (- (`GameplayStatics.GetTimeSeconds`) (`self.LastReceiveTime`)) 0.5)
        (`self.ChangeControlMode` 0)
        ;[1 1 1] 注释
        (`self.Reset`)
        (`KismetSystemLibrary.Delay` 0.1)
        (for (_ _array_index) (`self.LoopVar`)
          (`SimpleWheeledVehicleMovementComponent.SetBrakeTorque` (`self.SimpleWheeledVehicleMovement`) 0.0 _array_index))))
    (else
      (`self.PublishCmdVel` _linear_x (* -1 _angular_z)))))

(event `self.ReceiveTick`
  (params (DeltaSeconds :type "Float (single-precision)")))

(event `InputAction|IsHandling`
  (params (Key :type "Key Structure"))
  (:`Pressed`
    (if (!= (`self.ControlMode`) 2)
      (`self.ChangeControlMode` 1)))
  (:`Released`
    (`KismetSystemLibrary.Delay` 0.5)
    (if (!= (`self.ControlMode`) 2)
      (`self.ChangeControlMode` 0)
      ;[1 1 1] 注释
      (`self.Reset`)
      (`KismetSystemLibrary.Delay` 0.1)
      (for (_ _array_index) (`self.LoopVar`)
        (`SimpleWheeledVehicleMovementComponent.SetBrakeTorque` (`self.SimpleWheeledVehicleMovement`) 0.0 _array_index)))))

(event `InputAction|Handbrake`
  (params (Key :type "Key Structure"))
  (:`Pressed`
    (for (_ _array_index) (`self.LoopVar`)
      (`SimpleWheeledVehicleMovementComponent.SetBrakeTorque` (`self.SimpleWheeledVehicleMovement`) 2000.0 _array_index)))
  (:`Released`
    (for (_ _array_index_2) (`self.LoopVar`)
      (`SimpleWheeledVehicleMovementComponent.SetBrakeTorque` (`self.SimpleWheeledVehicleMovement`) 0.0 _array_index_2))))

(event `InputAxis|LookUp`
  (params (AxisValue :type "Float (single-precision)"))
  (`self.AddControllerPitchInput` AxisValue))

(event `InputAxis|LookRight`
  (params (AxisValue :type "Float (single-precision)"))
  (`self.AddControllerYawInput` AxisValue))

(event `/Game/UserInterface/MqttMessageClient.MessageReceived`
  (params (MqttMessage :type "MqttMessage Structure"))
  (bind (_message _topic) (break `MqttMessage` MqttMessage))
  (if (!= (`self.ControlMode`) 1)
    (if (`KismetStringLibrary.EqualEqual_StrStr` _topic "/publish/odom")
      (bind (_targetlinear _targetangular) (`self.ParseJson` _message))
      (set `self.TargetAngular` (* -1 _targetangular))
      (set `self.TargetLinear` (* 100 _targetlinear))
      (if (or (> (`KismetMathLibrary.Abs` (`self.TargetLinear`)) 5.0) (> (`KismetMathLibrary.Abs` (`self.TargetAngular`)) 0.1))
        (set `self.LastReceiveTime` (`GameplayStatics.GetTimeSeconds`))
        (if (!= (`self.ControlMode`) 2)
          (`self.ChangeControlMode` 2))))))

(fn `ChangeControlMode`
  (params (ControlMode :type Integer))
  (bind _output_get (set `self.ControlMode` ControlMode))
  (bind _foundwidgets (`WidgetBlueprintLibrary.GetAllWidgetsWithInterface` "/Game/UserInterface/MqttMessageServer.MqttMessageServer_C"))
  (for _array_element _foundwidgets
    (message `/Game/UserInterface/MqttMessageServer.PublishMessage` _array_element (make `MqttMessage` (`KismetStringLibrary.Conv_IntToString` _output_get) "/subscribe/mode"))))

(fn `Main`
  (bind (_angular_x _angular_y _angular_z) (`KismetMathLibrary.BreakVector` (`self.Angular`)))
  (`self.UpdateLinearAndAngular`)
  (`self.ShowFigure` _angular_z)
  (switch `int` (`self.ControlMode`)
    (:`0`)
    (:`1`
      (`self.SetTargetVel` (* (`self.GetInputAxisValue`) (`self.MaxLinear`)) (* (`self.GetInputAxisValue`) (`self.MaxAngular`))))
    (:`2`
      (`self.SetTargetVel` (`self.TargetLinear`) (`self.TargetAngular`)))))

(fn `ParseJson`
  (params (JsonString :type String))
  (returns (TargetLinear :type "Float (double-precision)") (TargetAngular :type "Float (double-precision)"))
  (bind _returnvalue (`VaRestSubsystem.DecodeJsonObject` (subsystem `VaRestSubsystem`) JsonString))
  (bind _returnvalue_2 (`VaRestJsonObject.GetObjectField` (`VaRestJsonObject.GetObjectField` _returnvalue "twist") "twist"))
  (return (`VaRestJsonObject.GetNumberField` (`VaRestJsonObject.GetObjectField` _returnvalue_2 "linear") "x") (`VaRestJsonObject.GetNumberField` (`VaRestJsonObject.GetObjectField` _returnvalue_2 "angular") "z")))

(fn `PidAdjustAngularTorque`
  (params (TargetAngular :type "Float (double-precision)"))
  (returns (AngularTorque :type "Float (double-precision)"))
  (bind _buffer_w (`self.Buffer_w`))
  (bind (_angular_x _angular_y _angular_z) (`KismetMathLibrary.BreakVector` (`self.Angular`)))
  (bind _output_get (set `self.Epw` (/ (- TargetAngular _angular_z) 1.0)))
  (`KismetArrayLibrary.Array_Insert` (`self.Buffer_w`) _output_get)
  (`KismetArrayLibrary.Array_Resize` (`self.Buffer_w`) 200)
  (set `self.Eiw` 0.0)
  (for _array_element (`self.Buffer_w`)
    (set `self.Eiw` (`self.LimitIn` 10.0 (+ _array_element (`self.Eiw`)) -10.0)))
  (set `self.Edw` (- (`|GetArrayItem` _buffer_w) (`|GetArrayItem` _buffer_w 1)))
  (return (+ (* (`self.Kpw`) (`self.Epw`)) (* (`self.Kiw`) (`self.Eiw`)) (* (`self.Kdw`) (`self.Edw`)))))

(fn `PidAdjustLinearTorque`
  (params (TargetLinear :type "Float (double-precision)"))
  (returns (LinearTorque :type "Float (double-precision)"))
  (bind _linear_x (`KismetMathLibrary.BreakVector` (`self.Linear`)))
  (bind _buffer_v (`self.Buffer_v`))
  (bind _output_get (set `self.Epv` (/ (- TargetLinear _linear_x) 250.0)))
  (`KismetArrayLibrary.Array_Insert` (`self.Buffer_v`) _output_get)
  (`KismetArrayLibrary.Array_Resize` (`self.Buffer_v`) 100)
  (set `self.Eiv` 0.0)
  (for _array_element (`self.Buffer_v`)
    (set `self.Eiv` (`self.LimitIn` 30.0 (+ _array_element (`self.Eiv`)) -30.0)))
  (set `self.Edv` (- (`|GetArrayItem` _buffer_v) (`|GetArrayItem` _buffer_v 1)))
  (return (+ (* (`self.Kpv`) (`self.Epv`)) (* (`self.Kiv`) (`self.Eiv`)) (* (`self.Kdv`) (`self.Edv`)))))

(fn `PublishCmdVel`
  (params (Linear :type "Float (double-precision)") (Angular :type "Float (double-precision)"))
  (bind _foundwidgets (`WidgetBlueprintLibrary.GetAllWidgetsWithInterface` "/Game/UserInterface/MqttMessageServer.MqttMessageServer_C"))
  (for _array_element _foundwidgets
    (message `/Game/UserInterface/MqttMessageServer.PublishMessage` _array_element (make `MqttMessage` (`KismetStringLibrary.Concat_StrStr` "{\"linear\":{\"x\":" (`KismetStringLibrary.Conv_DoubleToString` (/ Linear 100.0)) ",\"y\":0.0,\"z\":0.0},\"angular\":{\"x\":0.0,\"y\":0.0,\"z\":" (`KismetStringLibrary.Conv_DoubleToString` Angular) "}}") "/subscribe/cmd_vel"))))

(fn `Reset`
  (`self.SetDriveTorque` 0.0)
  (for (_ _array_index) (`self.LoopVar`)
    (`SimpleWheeledVehicleMovementComponent.SetBrakeTorque` (`self.SimpleWheeledVehicleMovement`) 200.0 _array_index)
    (`KismetArrayLibrary.Array_Clear` (`self.Buffer_v`))
    (`KismetArrayLibrary.Array_Clear` (`self.Buffer_w`))
    (set `self.TargetLinear` 0.0)
    (set `self.TargetAngular` 0.0)))

(fn `SetDriveTorque`
  (params (LinearTorque :type "Float (double-precision)") (AngularTorque :type "Float (double-precision)"))
  (for (_ _array_index) (`self.LoopVar`)
    (`SimpleWheeledVehicleMovementComponent.SetDriveTorque` (`self.SimpleWheeledVehicleMovement`) (+ LinearTorque (* (+ (* (mod _array_index 2) -2) 1) AngularTorque)) _array_index)))

(fn `SetTargetVel`
  (params (TargetLinear :type "Float (double-precision)") (TargetAngular :type "Float (double-precision)"))
  (`|ExecutionSequence`
    (:`then_0`
      (bind _lineartorque (`self.PidAdjustLinearTorque` TargetLinear)))
    (:`then_1`
      (bind _angulartorque (`self.PidAdjustAngularTorque` TargetAngular))
      (`self.SetDriveTorque` _lineartorque _angulartorque))))

(fn `ShowFigure`
  (params (Data :type "Float (double-precision) (by ref)"))
  (bind _datastring (`self.DataString`))
  (`self.UpdateList` Data)
  (set `self.DataString` "{\"series\":[{\"data\":[")
  (for (_array_element _array_index) (`self.DataList`)
    (if (== _array_index 99)
      (bind _returnvalue (`KismetStringLibrary.Conv_DoubleToString` _array_element))
      (set `self.DataString` (`KismetStringLibrary.Concat_StrStr` _datastring _returnvalue))
      (else
        (set `self.DataString` (`KismetStringLibrary.Concat_StrStr` _datastring _returnvalue ",")))))
  (bind _output_get (set `self.DataString` (`KismetStringLibrary.Concat_StrStr` (`self.DataString`) "]}]}")))
  (`WebInterface.Call` (`/Game/MyVehicle/Figure.WebUI` (`self.Figure`)) "ue2js" (`JsonLibraryHelpers.FromString` _output_get)))

(fn `UpdateLinearAndAngular`
  (bind _returnvalue (`PrimitiveComponent.GetPhysicsLinearVelocity` (`self.SkeletalMesh`) "None"))
  (set `self.Linear` (`KismetMathLibrary.GreaterGreater_VectorRotator` _returnvalue (* (`KismetMathLibrary.MakeRotFromX` (`SceneComponent.GetForwardVector` (`self.SkeletalMesh`))) -1)))
  (set `self.Angular` (`PrimitiveComponent.GetPhysicsAngularVelocityInRadians` (`self.SkeletalMesh`) "None")))

(fn `UpdateList`
  (params (Data :type "Float (double-precision) (by ref)"))
  (`KismetArrayLibrary.Array_Add` (`self.DataList`) Data)
  (`|ExecutionSequence`
    (:`then_0`
      (`KismetArrayLibrary.Array_Reverse` (`self.DataList`))
      (`KismetArrayLibrary.Array_Resize` (`self.DataList`) 100)
      (`KismetArrayLibrary.Array_Reverse` (`self.DataList`)))))

(fn `UserConstructionScript`)