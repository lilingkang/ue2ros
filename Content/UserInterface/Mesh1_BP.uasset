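; Actor that builds a procedural mesh colored as a stress heat map from the Baibi_cu vertex and Baibi_cu_index triangle DataTables.
; On BeginPlay it loads scaled positions, stress and reversed indices, then maps normalized stress to vertex hue from blue (low) to red (high).
; A half-second looping timer re-reads stress with random jitter and updates only the colors, simulating changing values.
; The construction script just clears data and assigns the material.
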(event `self.ReceiveBeginPlay`
  (`self.Get Data` 100.0)
  (`self.SetVertexColor`)
  (`ProceduralMeshComponent.CreateMeshSection_LinearColor` :`self` (`self.ProceduralMesh`) :`Vertices` (`self.Vertices`) :`Triangles` (`self.Triangles`) :`VertexColors` (`self.Vertex Colors`))
  (`KismetSystemLibrary.K2_SetTimerDelegate` (delegate `自定义事件_0`) 0.5 true))

(event `自定义事件_0`
  (`KismetArrayLibrary.Array_Clear` (`self.Stress`))
  (bind _outrownames (`DataTableFunctionLibrary.GetDataTableRowNames` "/Game/UserInterface/baibi_cu.baibi_cu"))
  (for _array_element _outrownames
    (bind _returnvalue (`|GetDataTableRow` "/Game/UserInterface/baibi_cu.baibi_cu" _array_element)
      (:`then`
        (`KismetArrayLibrary.Array_Add` (`self.Stress`) (* (`.stress_11_610721A84DB672FEC012D498106CB836` (break `/Game/UserInterface/Vertices` _returnvalue)) (`KismetMathLibrary.RandomFloatInRange` 0.5 1.5))))))
  (`KismetArrayLibrary.Array_Clear` (`self.Vertex Colors`))
  (`self.SetVertexColor`)
  (`ProceduralMeshComponent.UpdateMeshSection_LinearColor` :`self` (`self.ProceduralMesh`) :`Vertices` (`self.Vertices`) :`VertexColors` (`self.Vertex Colors`)))

(fn `ClearMeshData`
  (`KismetArrayLibrary.Array_Clear` (`self.Vertices`))
  (`KismetArrayLibrary.Array_Clear` (`self.Triangles`))
  (`KismetArrayLibrary.Array_Clear` (`self.Vertex Colors`))
  (`KismetArrayLibrary.Array_Clear` (`self.Stress`)))

(fn `Get Data`
  (params (Scale :type "Float (double-precision)" :default 0.0))
  (bind _scale (`local.Scale`))
  (`|ExecutionSequence`
    (:`then_0`
      ;[1 1 1] Get Vertices
      (bind _outrownames (`DataTableFunctionLibrary.GetDataTableRowNames` "/Game/UserInterface/baibi_cu.baibi_cu"))
      (for _array_element _outrownames
        (bind _returnvalue (`|GetDataTableRow` "/Game/UserInterface/baibi_cu.baibi_cu" _array_element)
          (:`then`
            (`|ExecutionSequence`
              (:`then_0`
                (bind (_x _y _z _stress) (break `/Game/UserInterface/Vertices` _returnvalue))
                (`KismetArrayLibrary.Array_Add` (`self.Vertices`) (`KismetMathLibrary.MakeVector` (* _x _scale) (* _y _scale) (* _z _scale))))
              (:`then_1`
                (`KismetArrayLibrary.Array_Add` (`self.Stress`) _stress)))))))
    (:`then_1`
      ;[1 1 1] Get Triangles
      (bind _outrownames_2 (`DataTableFunctionLibrary.GetDataTableRowNames` "/Game/UserInterface/baibi_cu_index.baibi_cu_index"))
      (for _array_element_2 _outrownames_2
        (bind _returnvalue_2 (`|GetDataTableRow` "/Game/UserInterface/baibi_cu_index.baibi_cu_index" _array_element_2)
          (:`then`
            (`KismetArrayLibrary.Array_Add` (`self.Triangles`) (`.index_2_5A0CAB79486A647DE40EF6A416A84BCB` (break `/Game/UserInterface/Triangles` _returnvalue_2))))))
      (`KismetArrayLibrary.Array_Reverse` (`self.Triangles`)))))

(fn `SetVertexColor`
  (bind (_indexofmaxvalue _maxvalue) (`KismetMathLibrary.MaxOfFloatArray` (`self.Stress`)))
  (for _array_element (`self.Stress`)
    (`KismetArrayLibrary.Array_Add` (`self.Vertex Colors`) (`KismetMathLibrary.HSVToRGB` (* (/ (- _maxvalue _array_element) (- _maxvalue (`.MinValue` (`KismetMathLibrary.MinOfFloatArray` (`self.Stress`))))) 240.0) 1.0 1.0))))

(fn `UserConstructionScript`
  (`self.ClearMeshData`)
  (`PrimitiveComponent.SetMaterial` (`self.ProceduralMesh`) 0 "/Game/UserInterface/Mesh1Material.Mesh1Material"))