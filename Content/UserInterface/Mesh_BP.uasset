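; Procedural mesh actor that builds a flat, vertical grid in the XZ plane at construction time, sized by XLength and YLength.
; DrawQuad generates evenly spaced vertices with normalized UVs, then derives triangles, normals and tangents through the built-in procedural mesh helpers.
; The construction script clears old data, creates the section with four fixed vertex colors and applies MyMaterial; the event graph is empty.
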(event `self.ReceiveBeginPlay`)

(fn `ClearMeshData`
  (`KismetArrayLibrary.Array_Clear` (`self.Vertices`))
  (`KismetArrayLibrary.Array_Clear` (`self.Triangles`))
  (`KismetArrayLibrary.Array_Clear` (`self.UV0`)))

(fn `DrawQuad`
  (locals (X :type Integer) (Y :type Integer))
  (for _index (range (+ (`self.XLength`) 1))
    (set `local.X` _index)
    (for _index_2 (range (+ (`self.YLength`) 1))
      (set `local.Y` _index_2)
      (`|ExecutionSequence`
        (:`then_0`
          ;[1 1 1] Make Vertex Locations
          (`KismetArrayLibrary.Array_Add` (`self.Vertices`) (`KismetMathLibrary.MakeVector` (* (`local.X`) 50.0) 0.0 (* (`local.Y`) 50.0))))
        (:`then_1`
          ;[1 1 1] Make UV Locations
          (`KismetArrayLibrary.Array_Add` (`self.UV0`) (`KismetMathLibrary.MakeVector2D` (/ (`KismetMathLibrary.Conv_IntToDouble` (`local.X`)) (`KismetMathLibrary.Conv_IntToDouble` (`self.XLength`))) (/ (`KismetMathLibrary.Conv_IntToDouble` (`local.Y`)) (`KismetMathLibrary.Conv_IntToDouble` (`self.YLength`)))))))))
  (`|ExecutionSequence`
    (:`then_0`
      ;[1 1 1] Create Triangles
      (bind _triangles (`KismetProceduralMeshLibrary.CreateGridMeshTriangles` (+ (`self.XLength`) 1) (+ (`self.YLength`) 1) true))
      (set `self.Triangles` _triangles))
    (:`then_1`
      ;[1 1 1] Tangents and Normals for Mesh
      (bind (_normals _tangents) (`KismetProceduralMeshLibrary.CalculateTangentsForMesh` (`self.Vertices`) (`self.Triangles`) (`self.UV0`)))
      (set `self.Normals` _normals)
      (set `self.Tangents` _tangents))))

(fn `UserConstructionScript`
  (`|ExecutionSequence`
    (:`then_0`
      (`self.ClearMeshData`)
      (`self.DrawQuad`))
    (:`then_1`
      (`ProceduralMeshComponent.CreateMeshSection_LinearColor` :`self` (`self.ProceduralMesh`) :`Vertices` (`self.Vertices`) :`Triangles` (`self.Triangles`) :`Normals` (`self.Normals`) :`UV0` (`self.UV0`) :`VertexColors` (`|MakeArray` (struct :`R` 1.0 :`G` 0.076389 :`B` 0.076389 :`A` 1.0) (struct :`G` 0.084157 :`B` 1.0 :`A` 1.0) (struct :`R` 0.059596 :`G` 1.0 :`A` 1.0) (struct :`R` 1.0 :`G` 0.862042 :`A` 1.0) :!type "LinearColor Structure") :`Tangents` (`self.Tangents`))
      (`PrimitiveComponent.SetMaterial` (`self.ProceduralMesh`) 0 "/Game/UserInterface/MyMaterial.MyMaterial"))))